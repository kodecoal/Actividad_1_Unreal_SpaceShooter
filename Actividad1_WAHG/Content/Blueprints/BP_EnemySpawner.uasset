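; BP_EnemySpawner endlessly spawns BP_EnemyPawn actors just above the visible screen of the orthographic player camera.
; On BeginPlay it takes the camera from BP_PlayerPawnSpace and derives horizontal Y limits and a top Z from its location, ortho width and aspect ratio.
; A delay loop then spawns an enemy at a random Y within those inset limits, ignoring collision, every SpawnDelay seconds.
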(event `self.ReceiveBeginPlay`
  (bind _asbp_player_pawn_space (cast `/Game/Blueprints/BP_PlayerPawnSpace` (`GameplayStatics.GetPlayerPawn` 0)))
  (`self.Set Viewport Limits` (`/Game/Blueprints/BP_PlayerPawnSpace.Player Camera Reference` _asbp_player_pawn_space))
  (`self.Spawn Enemy` :!label _label)
  (`KismetSystemLibrary.Delay` (`self.Spawn Delay`))
  (goto _label))

(event `Spawn Enemy`
  ; Para hacer que los enenmigos aparezcan de forma aleatoria
  (`|SpawnActorFromClass` "/Game/Blueprints/BP_EnemyPawn.BP_EnemyPawn_C" (`KismetMathLibrary.MakeTransform` (`KismetMathLibrary.MakeVector` 0.0 (+ (`KismetMathLibrary.RandomFloatInRange` (`self.Y Min`) (`self.Y Max`)) 2.0) (`self.Z Spawn`))) "AlwaysSpawn" "MultiplyWithRoot" null null))

(event `Set Viewport Limits`
  (params (Camera :type "CameraComponent Object Reference"))
  (bind _returnvalue (`SceneComponent.K2_GetComponentLocation` Camera))
  (bind _orthowidth (`CameraComponent.OrthoWidth` Camera))
  (bind (_returnvalue_x _returnvalue_y) (`KismetMathLibrary.BreakVector` (- _returnvalue (* (* _orthowidth 0.5) (0.0 1.0 0.0)))))
  (bind (_returnvalue_x_2 _returnvalue_y_2 _returnvalue_z) (`KismetMathLibrary.BreakVector` (+ _returnvalue (* (* (/ _orthowidth (`CameraComponent.AspectRatio` Camera)) 0.5) (0.0 0.0 1.0)))))
  ; Calculo para hacer aparecer a diferentes enenmigos en la pantalla
  (bind _output_get (set `self.Y Min` (+ _returnvalue_y 50.0)))
  (set `self.Y Max` (- (+ _output_get _orthowidth) 100.0))
  (set `self.Z Spawn` (+ _returnvalue_z 50.0)))

(fn `UserConstructionScript`)