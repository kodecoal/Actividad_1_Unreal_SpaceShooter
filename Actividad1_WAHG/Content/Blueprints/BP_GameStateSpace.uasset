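; BP_GameStateSpace is a game state Blueprint that tracks score and game-over status, apparently for a space game.
; On BeginPlay it creates the WBP_MainUI widget for player controller 0, keeps a reference and adds it to the viewport.
; IncreaseScore adds a given point value to Score.
; GameOver sets the IsGameOver flag and tells the main UI to show its game-over display.
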(event `self.ReceiveBeginPlay`
  (bind _returnvalue (`|CreateWidget` "/Game/Blueprints/WBP_MainUI.WBP_MainUI_C" (`GameplayStatics.GetPlayerController` 0)))
  (bind _output_get (set `self.Main UI` _returnvalue))
  (`UserWidget.AddToViewport` _output_get 0))

(event `Increase Score`
  (params (`Point Value` :type Integer))
  ; Incrementa el score en el tablero
  (set `self.Score` (+ `Point Value` (`self.Score`))))

(event `Game Over`
  (set `self.Is Game Over?` true)
  (`/Game/Blueprints/WBP_MainUI.Show Game Over Ui` (`self.Main UI`)))

(fn `UserConstructionScript`)