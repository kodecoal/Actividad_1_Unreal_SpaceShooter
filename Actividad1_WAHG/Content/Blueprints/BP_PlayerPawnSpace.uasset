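; BP_PlayerPawnSpace is a player ship pawn that follows the mouse along the world Y axis and fires lasers.
; On BeginPlay it caches the sprite's starting Z.
; Each Tick deprojects the mouse position to world space and moves the ship sprite to that Y, holding X at zero and Z at the cached height.
; The IA_FireLaser input action spawns a BP_Laser at the sprite's location.
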(event `self.ReceiveBeginPlay`
  (`self.Get Vertical Position`))

(event `self.ReceiveTick`
  (params (DeltaSeconds :type "Float (single-precision)"))
  (bind _returnvalue (`self.GetLocalViewingPlayerController`))
  (bind (_locationx _locationy) (`PlayerController.GetMousePosition` _returnvalue))
  ; Mueve al player con el mouse solo en el eje Y, si quiero que se mueva por toda la pantalla conecto el eje Z en el Break Vector al Make Vector
  (`SceneComponent.K2_SetWorldLocation` (`self.playerShip2_red_Sprite`) (`KismetMathLibrary.MakeVector` 0.0 (.y (`PlayerController.DeprojectScreenPositionToWorld` _returnvalue _locationx _locationy)) (`self.Start Z Position`)) false false))

(event `Fire Laser`
  (`|SpawnActorFromClass` "/Game/Blueprints/BP_Laser.BP_Laser_C" (`KismetMathLibrary.Conv_VectorToTransform` (`SceneComponent.K2_GetComponentLocation` (`self.playerShip2_red_Sprite`))) "Undefined" "MultiplyWithRoot" null null))

(event `EnhancedInput|/Game/Blueprints/IA_FireLaser`
  (params (ActionValue :type Boolean) (ElapsedSeconds :type "Float (double-precision)") (TriggeredSeconds :type "Float (double-precision)") (InputAction :type "InputAction Object Reference" :default "/Game/Blueprints/IA_FireLaser.IA_FireLaser"))
  (:`Triggered`
    (`self.Fire Laser`)))

(fn `Get Vertical Position`
  (bind (_returnvalue_x _returnvalue_y _returnvalue_z) (`KismetMathLibrary.BreakVector` (`SceneComponent.K2_GetComponentLocation` (`self.playerShip2_red_Sprite`))))
  ; Para conocer la posición del player en el eje Z
  (set `self.Start Z Position` _returnvalue_z))

(fn `UserConstructionScript`
  (set `self.Player Camera Reference` (`self.Camera`)))