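; BP_EnemyPawn is an enemy pawn for a space game that moves along negative Z at its Speed each tick.
; On BeginPlay it caches the BP_GameStateSpace game state.
; Overlapping an actor tagged Player calls GameOver, while any other overlap adds PointValue to the score.
; In both cases it destroys the other actor and itself.
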(event `self.ReceiveBeginPlay`
  (bind _asbp_game_state_space (cast `/Game/Blueprints/BP_GameStateSpace` (`GameplayStatics.GetGameState`)))
  (set `self.Current Game State` _asbp_game_state_space))

(event `self.ReceiveTick`
  (params (DeltaSeconds :type "Float (single-precision)"))
  ; Es la veloscidad del enenmigo, solo que para no lidear con una velocidad en enegativo cvolvemos a multiplicar por -1
  (`self.K2_AddActorWorldOffset` (`KismetMathLibrary.MakeVector` 0.0 0.0 (* (* DeltaSeconds (`self.Speed`)) -1.0))))

(event `self.ReceiveActorBeginOverlap`
  (params (OtherActor :type "Actor Object Reference"))
  (bind _current_game_state (`self.Current Game State`))
  (if (`self.ActorHasTag` OtherActor "Player")
    (`/Game/Blueprints/BP_GameStateSpace.Game Over` _current_game_state)
    (else
      (`/Game/Blueprints/BP_GameStateSpace.Increase Score` _current_game_state (`self.Point Value`))))
  (`self.K2_DestroyActor` OtherActor)
  (`self.K2_DestroyActor`))

(fn `UserConstructionScript`)